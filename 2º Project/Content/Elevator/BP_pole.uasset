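; BP_pole is an elevator control pole that lets the player operate the level's BP_Elevator when nearby.
; A box overlap with BP_Sorcerer toggles input, a prompt widget and the Active flag.
; The Elevator action alternates ElevatorUp and ElevatorDown on the elevator found at BeginPlay.
; Separately, the F key alternates two timelines that rotate the Arrow around its roll axis, with its own FlipFlop.
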(event `self.Box1.OnComponentBeginOverlap`
  (params (OverlappedComponent :type "PrimitiveComponent Object Reference") (OtherActor :type "Actor Object Reference") (OtherComp :type "PrimitiveComponent Object Reference") (OtherBodyIndex :type Integer) (bFromSweep :type Boolean) (SweepResult :type "HitResult Structure (by ref)"))
  (cast `/Game/Character/BP_Sorcerer` OtherActor)
  (`self.EnableInput` (`GameplayStatics.GetPlayerController` 0))
  (`SceneComponent.SetVisibility` (`self.Widget`) true false)
  (set `self.active` true))

(event `self.Box1.OnComponentEndOverlap`
  (params (OverlappedComponent :type "PrimitiveComponent Object Reference") (OtherActor :type "Actor Object Reference") (OtherComp :type "PrimitiveComponent Object Reference") (OtherBodyIndex :type Integer))
  (cast `/Game/Character/BP_Sorcerer` OtherActor)
  (`self.DisableInput` (`GameplayStatics.GetPlayerController` 0))
  (`SceneComponent.SetVisibility` (`self.Widget`) false false)
  (set `self.active` false))

(event `InputAction|Elevator`
  (params (Key :type "Key Structure"))
  (bind _elevator (`self.Elevator`))
  (:`Pressed`
    (if (`self.active`)
      (`/Engine/EditorBlueprintResources/StandardMacros.FlipFlop`
        (:`A`
          (`/Game/Elevator/BP_Elevator.ElevatorUp` _elevator))
        (:`B`
          (`/Game/Elevator/BP_Elevator.ElevatorDown` _elevator))))))

(event `self.ReceiveBeginPlay`
  (bind _returnvalue (`GameplayStatics.GetActorOfClass` "/Game/Elevator/BP_Elevator.BP_Elevator_C"))
  (set `self.Elevator` _returnvalue))

(event `Key|F`
  (params (Key :type "Key Structure"))
  (bind _arrow (`self.Arrow`))
  (:`Pressed`
    (`/Engine/EditorBlueprintResources/StandardMacros.FlipFlop`
      (:`A`
        (bind (_direction _rotationx) (`Timeline|Timeline_0` :!via `PlayFromStart`)
          (:`Update`
            (`SceneComponent.K2_SetRelativeRotation` _arrow (`KismetMathLibrary.MakeRotator` _rotationx) false false))))
      (:`B`
        (bind (_direction_2 _rotationx_2) (`Timeline|Timeline` :!via `PlayFromStart`)
          (:`Update`
            (`SceneComponent.K2_SetRelativeRotation` _arrow (`KismetMathLibrary.MakeRotator` _rotationx_2) false false)))))))

(fn `UserConstructionScript`)