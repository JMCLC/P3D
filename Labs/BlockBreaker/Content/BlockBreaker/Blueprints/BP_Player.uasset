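; BP_Player is the first-person player of BlockBreaker, handling movement, mouse-style look and shooting with a rifle.
; On BeginPlay it spawns a BP_Rifle, stores it as EquippedGun and snaps it to the GunLocation component.
; Axis inputs drive movement and controller rotation, with inverted pitch input.
; Holding Shoot passes a camera-forward line to the gun's Shoot, rate-limited by a CanShoot flag and a Delay from the gun's FireRate.
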(event `self.ReceiveBeginPlay`
  (bind _returnvalue (`|SpawnActorFromClass` "/Game/BlockBreaker/Blueprints/BP_Rifle.BP_Rifle_C" (`KismetMathLibrary.MakeTransform` (0.0 0.0 0.0)) "Undefined" "MultiplyWithRoot" null null))
  (bind _output_get (set `self.EquippedGun` _returnvalue))
  (`self.K2_AttachToComponent` _output_get (`self.GunLocation`) "None" "SnapToTarget" "SnapToTarget" "SnapToTarget" true))

(event `InputAxis|MoveForward`
  (params (AxisValue :type "Float (single-precision)"))
  (`self.AddMovementInput` (`self.GetActorForwardVector`) AxisValue))

(event `InputAxis|Shoot`
  (params (AxisValue :type "Float (single-precision)"))
  (bind _fpscamera (`self.FPSCamera`))
  (bind _returnvalue (`SceneComponent.K2_GetComponentLocation` _fpscamera))
  (if (and (== AxisValue 1.0) (`self.CanShoot`))
    (`/Game/BlockBreaker/Blueprints/BP_BaseGun.Shoot` (`self.EquippedGun`) _returnvalue (+ _returnvalue (* (`SceneComponent.GetForwardVector` _fpscamera) (`/Game/BlockBreaker/Blueprints/BP_BaseGun.MaxBulletDistance` (`self.EquippedGun`)))))
    (set `self.CanShoot` false)
    (`KismetSystemLibrary.Delay` (`/Game/BlockBreaker/Blueprints/BP_BaseGun.FireRate` (`self.EquippedGun`)))
    (set `self.CanShoot` true)))

(event `InputAxis|MoveRight`
  (params (AxisValue :type "Float (single-precision)"))
  (`self.AddMovementInput` (`self.GetActorRightVector`) AxisValue))

(event `InputAxis|LookHorizontal`
  (params (AxisValue :type "Float (single-precision)"))
  (`self.AddControllerYawInput` AxisValue))

(event `InputAxis|LookVertical`
  (params (AxisValue :type "Float (single-precision)"))
  (`self.AddControllerPitchInput` (* AxisValue -1.0)))

(fn `UserConstructionScript`)